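; BP_Player is the player-controlled cube that moves forward on its own while the player steers it side to side.
; Tick applies a constant-variable forward force on X, and the MoveLeftRight axis scales SideForce along Y.
; Both pushes run only while LevelInPlay is true and use physics AddForce as an acceleration change, so mass does not affect them.
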(event `self.ReceiveTick`
  (params (DeltaSeconds :type "Float (single-precision)"))
  ;[0.1816 1 0.1744] Event Tick
  (`|ExecutionSequence`
    (:`then_0`
      ;[0.1816 1 0.1744] Should Forward Motion be Applied? (Level In Play)
      (if (`self.bLevelInPlay`)
        ;[0.1816 1 0.1744] Apply Forward Force (Acceleration)
        (`PrimitiveComponent.AddForce` (`self.Cube`) (`KismetMathLibrary.MakeVector` (`self.Force X`)) "None" true)))))

(event `InputAxis|MoveLeftRight`
  (params (AxisValue :type "Float (single-precision)"))
  ;[0.1816 1 0.1744] Player Controlled Side to Side Motion
  (if (`self.bLevelInPlay`)
    (`PrimitiveComponent.AddForce` (`self.Cube`) (`KismetMathLibrary.MakeVector` 0.0 (* (`self.GetInputAxisValue`) (`self.SideForce`))) "None" true)))

(fn `UserConstructionScript`)